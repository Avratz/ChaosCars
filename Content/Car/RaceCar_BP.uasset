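; Player race car pawn that handles driving, lap counting and the race HUD.
; On BeginPlay it counts TrackCheckpoints, creates MainUI and holds throttle for a three-second countdown.
; Enhanced Input feeds the vehicle movement component, while mouse axes rotate the spring arm.
; Overlaps advance checkpoints in index order; checkpoint 0 after the last adds a lap without resetting CurrentCheckpoint, and reaching TotalLaps shows the win and disables throttle.
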(event `self.ReceiveBeginPlay`
  (bind _asplayer_controller (cast `PlayerController` (`self.GetController`)))
  (message `EnhancedInputSubsystemInterface.AddMappingContext` (pcsubsystem `EnhancedInputLocalPlayerSubsystem` _asplayer_controller) "/Game/Input/MainInputMap.MainInputMap" 0 (struct))
  (bind _outactors (`GameplayStatics.GetAllActorsOfClass` "/Game/Blueprints/TrackCheckpoint.TrackCheckpoint_C"))
  (set `self.CheckpointCount` (`KismetArrayLibrary.Array_Length` _outactors))
  (bind _returnvalue (`|GenericCreateObject` "/Game/Blueprints/MainUI.MainUI_C"))
  (bind _output_get (set `self.UI` _returnvalue))
  (`UserWidget.AddToViewport` _output_get 0)
  (`/Game/Blueprints/MainUI.UpdateLapText` _output_get (`self.CurrentLap`) (`self.TotalLaps`))
  (`/Game/Blueprints/MainUI.RaceStartTimer` _output_get)
  (set `self.CanThrottle` false)
  (`KismetSystemLibrary.Delay` 3.0)
  (set `self.CanThrottle` true))

(event `self.ReceiveActorBeginOverlap`
  (params (OtherActor :type "Actor Object Reference"))
  (bind _totallaps (`self.TotalLaps`))
  (bind _ui (`self.UI`))
  (bind _astrack_checkpoint (cast `/Game/Blueprints/TrackCheckpoint` OtherActor))
  (bind _checkpointindex (`/Game/Blueprints/TrackCheckpoint.CheckpointIndex` _astrack_checkpoint))
  (if (== _checkpointindex (+ (`self.CurrentCheckpoint`) 1))
    (set `self.CurrentCheckpoint` _checkpointindex)
    (elif (and (== _checkpointindex 0) (== (`self.CurrentCheckpoint`) (- (`self.CheckpointCount`) 1)))
      (bind _output_get (set `self.CurrentLap` (+ (`self.CurrentLap`) 1)))
      (`/Game/Blueprints/MainUI.UpdateLapText` _ui _output_get _totallaps)
      (if (== _output_get _totallaps)
        (`/Game/Blueprints/MainUI.WinGame` _ui)
        (set `self.CanThrottle` false)))))

(event `EnhancedInput|/Game/Input/Throttle`
  (params (ActionValue :type "Float (double-precision)") (ElapsedSeconds :type "Float (double-precision)") (TriggeredSeconds :type "Float (double-precision)") (InputAction :type "InputAction Object Reference" :default "/Game/Input/Throttle.Throttle"))
  (:`Triggered`
    (if (`self.CanThrottle`) :!label _label
      (`ChaosVehicleMovementComponent.SetThrottleInput` (`self.VehicleMovementComponent`) ActionValue)))
  (:`Completed`
    (goto _label)))

(event `InputAxisKey|MouseX`
  (params (AxisValue :type "Float (single-precision)"))
  (`SceneComponent.K2_AddRelativeRotation` (`self.SpringArm`) (`KismetMathLibrary.MakeRotator` 0.0 0.0 AxisValue) false false))

(event `EnhancedInput|/Game/Input/Break`
  (params (ActionValue :type "Float (double-precision)") (ElapsedSeconds :type "Float (double-precision)") (TriggeredSeconds :type "Float (double-precision)") (InputAction :type "InputAction Object Reference" :default "/Game/Input/Break.Break"))
  (:`Triggered`
    (`ChaosVehicleMovementComponent.SetBrakeInput` (`self.VehicleMovementComponent`) ActionValue :!label _label_2))
  (:`Completed`
    (goto _label_2)))

(event `InputAxisKey|MouseY`
  (params (AxisValue :type "Float (single-precision)"))
  (`SceneComponent.K2_AddRelativeRotation` (`self.SpringArm`) (`KismetMathLibrary.MakeRotator` 0.0 AxisValue) false false))

(event `EnhancedInput|/Game/Input/HandBreak`
  (params (ActionValue :type Boolean) (ElapsedSeconds :type "Float (double-precision)") (TriggeredSeconds :type "Float (double-precision)") (InputAction :type "InputAction Object Reference" :default "/Game/Input/HandBreak.HandBreak"))
  (bind _vehiclemovementcomponent (`self.VehicleMovementComponent`))
  (:`Started`
    (`ChaosVehicleMovementComponent.SetHandbrakeInput` _vehiclemovementcomponent true))
  (:`Completed`
    (`ChaosVehicleMovementComponent.SetHandbrakeInput` _vehiclemovementcomponent false)))

(event `EnhancedInput|/Game/Input/Steering`
  (params (ActionValue :type "Float (double-precision)") (ElapsedSeconds :type "Float (double-precision)") (TriggeredSeconds :type "Float (double-precision)") (InputAction :type "InputAction Object Reference" :default "/Game/Input/Steering.Steering"))
  (:`Triggered`
    (`ChaosVehicleMovementComponent.SetSteeringInput` (`self.VehicleMovementComponent`) ActionValue :!label _label_3))
  (:`Completed`
    (goto _label_3)))

(fn `UserConstructionScript`)